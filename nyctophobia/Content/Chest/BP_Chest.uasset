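; BP_Chest is an interactable chest that opens on interaction unless its Lock flag is set.
; Opening plays a sound, waits briefly, then plays the open animation and disables actor collision, with DoOnce guards limiting it to a single run.
; The locked path only keeps Lock set, with no feedback.
; Box collision overlaps show and hide a widget as actors enter and leave.
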(event `/Game/ThirdPerson/Blueprints/Interaction_Interface.Interaction`
  (params (Actor :type "Actor Object Reference"))
  (if (`self.Lock?`)
    (`self.Can't Open Chest`)
    (else
      (`self.Open Chest`))))

(event `Open Chest`
  ;[1 1 1] Open Chest
  (set `self.Lock?` false)
  (`/Engine/EditorBlueprintResources/StandardMacros.DoOnce` false
    (:`Completed`
      (`GameplayStatics.PlaySoundAtLocation` "/Game/SoundEffect/SFX/Open_Chest.Open_Chest" (`SceneComponent.K2_GetComponentLocation` (`self.Chest`)) (struct) 1.0 1.0 0.0 null null null null)
      (`KismetSystemLibrary.Delay` 0.2)
      (`/Engine/EditorBlueprintResources/StandardMacros.DoOnce` false
        (:`Completed`
          (`SkeletalMeshComponent.PlayAnimation` (`self.Chest`) "/Game/Chest/Chest_Anim_Armature_A_Open.Chest_Anim_Armature_A_Open" false)
          (`self.SetActorEnableCollision` false))))))

(event `Can't Open Chest`
  ;[1 1 1] Cant Open Chest
  (set `self.Lock?` true))

(event `self.BoxCollision.OnComponentBeginOverlap`
  (params (OverlappedComponent :type "PrimitiveComponent Object Reference") (OtherActor :type "Actor Object Reference") (OtherComp :type "PrimitiveComponent Object Reference") (OtherBodyIndex :type Integer) (bFromSweep :type Boolean) (SweepResult :type "HitResult Structure (by ref)"))
  (bind _output_get (set `self.Widget` (`self.Widget`)))
  (`SceneComponent.SetVisibility` _output_get true false))

(event `self.BoxCollision.OnComponentEndOverlap`
  (params (OverlappedComponent :type "PrimitiveComponent Object Reference") (OtherActor :type "Actor Object Reference") (OtherComp :type "PrimitiveComponent Object Reference") (OtherBodyIndex :type Integer))
  (bind _output_get (set `self.Widget` (`self.Widget`)))
  (`SceneComponent.SetVisibility` _output_get false false))

(fn `UserConstructionScript`)