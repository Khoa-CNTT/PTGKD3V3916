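; Enemy AI pawn that spots the player and performs a melee catch attack.
; Pawn sensing detects actors tagged Player, raises walk speed and sets the seeingPlayer blackboard flag, with no reset here.
; AttackPlayer plays the Catching montage and immediately sphere-traces ahead of AttackTracePoint, damaging the hit pawn with a devil laugh.
; An Attacking flag blocks re-entry until the montage completes; the trace draws debug shapes.
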(event `self.PawnSensing.OnSeePawn`
  (params (Pawn :type "Pawn Object Reference"))
  ;[1 1 1] See Player
  (if (`self.ActorHasTag` Pawn "Player")
    (set `CharacterMovementComponent.MaxWalkSpeed` 650.0 (`self.CharacterMovement`))
    (`BlackboardComponent.SetValueAsBool` (`AIBlueprintHelperLibrary.GetBlackboard` (`AIBlueprintHelperLibrary.GetAIController` self)) "seeingPlayer" true)))

(event `Attack Player`
  (bind _attack_trace_point (`self.Attack Trace Point`))
  (bind _returnvalue (`SceneComponent.K2_GetComponentLocation` _attack_trace_point))
  ;[1 1 1] Attack Player
  (if (not (`self.attacking?`))
    (set `self.attacking?` true)
    (`|PlayMontage` (`self.Mesh`) "/Game/AI/Catching.Catching"
      (:`then`
        (bind (_outhit _returnvalue_2) (`KismetSystemLibrary.SphereTraceSingleForObjects` :`Start` _returnvalue :`End` (+ _returnvalue (* (`KismetMathLibrary.GetForwardVector` (`SceneComponent.K2_GetComponentRotation` _attack_trace_point)) 70.0)) :`Radius` 25.0 :`ObjectTypes` (`|MakeArray` "ObjectTypeQuery3" :!type "EObjectTypeQuery Enum") :`DrawDebugType` "ForDuration"))
        (if _returnvalue_2
          (`GameplayStatics.PlaySound2D` "/Game/SoundEffect/SFX/Devil_Laugh.Devil_Laugh" 1.0 1.0 0.0 null null)
          (`GameplayStatics.ApplyDamage` (`.HitActor` (`GameplayStatics.BreakHitResult` _outhit)) 10.0)))
      (:`OnCompleted`
        (set `self.attacking?` false)))))

(fn `UserConstructionScript`)