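; BP_Dial is a single ten-digit dial for a combination lock puzzle that starts on a random number.
; On BeginPlay it passes itself to its WB_Arrow widget and randomizes its rotation.
; RotateDial plays a click and uses a timeline to turn the mesh one step, with a flag blocking input mid-turn.
; When the turn finishes, it wraps the angle, derives Number from it and tells LockRef to check the combination.
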(event `self.ReceiveBeginPlay`
  (bind _aswb_arrow (cast `/Game/Lock_Puzzle/WB_Arrow` (`WidgetComponent.GetUserWidgetObject` (`self.Arrow`))))
  (`/Game/Lock_Puzzle/WB_Arrow.Innitialize` _aswb_arrow self)
  (`self.SetRandomNumber`))

(event `Find Number`
  (set `self.Number` (`KismetMathLibrary.FTrunc` (/ (`self.DialRotation`) 36.0))))

(event `Rotate Dial`
  (if (`self.CanRotate`)
    (set `self.CanRotate` false)
    (`GameplayStatics.PlaySound2D` "/Game/Lock_Puzzle/CombinationLockClick.CombinationLockClick" 1.0 1.0 0.0 null null)
    (bind (_direction _alpha) (`Timeline|DialRotateTL`)
      (:`Update`
        (bind _returnvalue (+ (`self.DialRotation`) (`KismetMathLibrary.Lerp` 0.0 36.0 _alpha)))
        (`SceneComponent.K2_SetRelativeRotation` (`self.SM_Dial`) (`KismetMathLibrary.MakeRotator` 0.0 0.0 _returnvalue) false false))
      (:`Finished`
        (set `self.DialRotation` _returnvalue)
        (if (>= (`self.DialRotation`) 360.0)
          (set `self.DialRotation` 0.0)
          (`SceneComponent.K2_SetRelativeRotation` :`self` (`self.SM_Dial`)))
        (`self.Find Number`)
        (`/Game/Lock_Puzzle/BP_LockCombi.Check Every Turn` (`self.LockRef`))
        (set `self.CanRotate` true)))))

(fn `SetRandomNumber`
  (bind _output_get (set `self.LocalRotation` (* (`KismetMathLibrary.RandomIntegerInRange` 0 9) 36.0)))
  (`SceneComponent.K2_SetRelativeRotation` (`self.SM_Dial`) (`KismetMathLibrary.MakeRotator` 0.0 0.0 _output_get) false false)
  (set `self.DialRotation` (`self.LocalRotation`))
  (`self.Find Number`))

(fn `UserConstructionScript`)