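; Three-dial combination lock puzzle that unlocks a referenced chest.
; BeginPlay spawns BP_Dial actors on mesh sockets, passing each an index and lock reference.
; Interaction blends to the lock's view, freezes the player and shows a cursor and notice widget; clicks forward through WidgetInteraction, and Escape or Q exits.
; CheckEveryTurn compares dials to LockCombination; a match plays sound and timeline drop, restores the player view, unlocks ChestRef and destroys lock and dials.
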(event `self.ReceiveBeginPlay`
  (for _index (range 3)
    (bind _returnvalue (`|SpawnActorFromClass` "/Game/Lock_Puzzle/BP_Dial.BP_Dial_C" (`KismetMathLibrary.MakeTransform` (0.0 0.0 0.0)) "Undefined" "MultiplyWithRoot" null _index self null))
    (`KismetArrayLibrary.Array_Add` (`self.Dials`) _returnvalue)
    (`self.K2_AttachToComponent` _returnvalue (`self.SM_CombinationLock`) (select `int` _index :`0` "Dial01" :`1` "Dial02" :`2` "Dial03" :!type "Name") "KeepRelative" "KeepRelative" "KeepRelative" true)
    (`self.EnableInput` self (`GameplayStatics.GetPlayerController` 0))))

(event `/Game/ThirdPerson/Blueprints/Interaction_Interface.Interaction`
  (params (Actor :type "Actor Object Reference"))
  (bind _returnvalue (`GameplayStatics.GetPlayerController` 0))
  ;[1 1 1] Interaction
  (`PlayerController.SetViewTargetWithBlend` (`GameplayStatics.GetPlayerController` 0) self 0.5 "VTBlend_Linear" 0.0 false)
  (bind _returnvalue_2 (`|CreateWidget` "/Game/UI/Notice_WB/WB_Notice_Lock.WB_Notice_Lock_C"))
  (`UserWidget.AddToViewport` _returnvalue_2 0)
  (`CharacterMovementComponent.DisableMovement` (`Character.CharacterMovement` (`GameplayStatics.GetPlayerCharacter` 0)))
  (`Controller.SetIgnoreLookInput` _returnvalue true)
  (`KismetSystemLibrary.Delay` 0.5)
  (`self.EnableInput` _returnvalue null)
  (set `PlayerController.bShowMouseCursor` true _returnvalue))

(event `Exit View`
  (bind _returnvalue (`GameplayStatics.GetPlayerController` 0))
  (bind _returnvalue_2 (`GameplayStatics.GetPlayerCharacter` 0))
  ;[1 1 1] Exit View
  (`PlayerController.SetViewTargetWithBlend` _returnvalue _returnvalue_2 0.5 "VTBlend_Linear" 0.0 false)
  (`self.DisableInput` _returnvalue null)
  (`Controller.ResetIgnoreLookInput` _returnvalue)
  (set `PlayerController.bShowMouseCursor` false _returnvalue)
  (`CharacterMovementComponent.SetMovementMode` (`Character.CharacterMovement` _returnvalue_2) "MOVE_Walking" 0))

(event `Key|Escape`
  (params (Key :type "Key Structure"))
  ;[1 1 1] Out View Key
  (:`Pressed`
    (`self.Exit View` :!label _label)))

(event `Key|LeftMouseButton`
  (params (Key :type "Key Structure"))
  (bind _widgetinteraction (`self.WidgetInteraction`))
  ;[1 1 1] Press key
  (:`Pressed`
    (`WidgetInteractionComponent.PressPointerKey` _widgetinteraction "LeftMouseButton"))
  (:`Released`
    (`WidgetInteractionComponent.ReleasePointerKey` _widgetinteraction "LeftMouseButton")))

(event `Key|Q`
  (params (Key :type "Key Structure"))
  ;[1 1 1] Out View Key
  (:`Pressed`
    (goto _label)))

(event `Check Every Turn`
  (bind _success (`self.Check Code`))
  (if _success
    (`self.Unlock Lock`)))

(event `Unlock Lock`
  ;[1 1 1] Unlock
  (`GameplayStatics.PlaySound2D` "/Game/Lock_Puzzle/CombinationLock_Unlock.CombinationLock_Unlock" 1.0 1.0 0.0 null null)
  (bind (_direction _alpha) (`Timeline|UnlockTL`)
    (:`Update`
      (`SceneComponent.K2_SetRelativeLocation` (`self.SM_CombinationLock`) (`KismetMathLibrary.MakeVector` 0.0 0.0 (`KismetMathLibrary.Lerp` 0.0 -4.0 _alpha)) false false)
      (`KismetSystemLibrary.Delay` 1.0)
      (`self.Exit View`)
      (set `/Game/Chest/BP_Chest.Lock?` false (`self.Chest Ref`))
      (`self.K2_DestroyActor` (`self.Dials`))
      (`self.K2_DestroyActor`))))

(fn `Check Code`
  (returns (Success :type Boolean))
  (locals (`Local Success` :type Boolean))
  (for (_array_element _array_index) (`self.Dials`)
    (if (== (`/Game/Lock_Puzzle/BP_Dial.Number` _array_element) (`|GetArrayItem` (`self.LockCombination`) _array_index))
      (set `local.Local Success` true)
      (else
        (set `local.Local Success` false)
        (break))))
  (return (`local.Local Success`)))

(fn `UserConstructionScript`)