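; BP_LightButton1 is an interactable light button in the lighting game that cycles a point light through a fixed set of colors.
; Each Interaction event plays a press sound, increments ColorIndex and wraps it to zero past the last color.
; UpdateLightColor then switches on that index to set the PointLight to white, red, orange or green.
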(event `/Game/ThirdPerson/Blueprints/Interaction_Interface.Interaction`
  (params (Actor :type "Actor Object Reference"))
  (`GameplayStatics.PlaySound2D` "/Game/SoundEffect/ChangePress.ChangePress" 1.0 1.0 0.0 null null)
  (bind _result (`/Engine/EditorBlueprintResources/StandardMacros.IncrementInt` (`self.ColorIndex`))
    (:`  `
      (if (not (<= _result 3))
        (set `self.ColorIndex` 0))
      (`self.Update Light Color`))))

(fn `Update Light Color`
  (switch `int` (`self.ColorIndex`)
    (:`0`
      (`LightComponent.SetLightColor` (`self.PointLight`) (struct :`R` 1.0 :`G` 1.0 :`B` 1.0 :`A` 1.0) true))
    (:`1`
      (`LightComponent.SetLightColor` (`self.PointLight`) (struct :`R` 0.932 :`A` 1.0) true))
    (:`2`
      (`LightComponent.SetLightColor` (`self.PointLight`) (struct :`R` 1.0 :`G` 0.443831 :`B` 0.076 :`A` 1.0) true))
    (:`3`
      (`LightComponent.SetLightColor` (`self.PointLight`) (struct :`R` 0.06591 :`G` 0.876 :`A` 1.0) true))))

(fn `UserConstructionScript`)