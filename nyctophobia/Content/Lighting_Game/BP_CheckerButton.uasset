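; BP_CheckerButton is an interactable button that checks a light color puzzle and triggers a linked door.
; On interaction it compares each puzzle piece's ColorIndex to ColorCode at the same position.
; A match messages DoortoOpen once through Interaction_Interface; a mismatch resets every piece's color and plays an error sound per piece.
; Sphere overlap toggles a widget's visibility, adding a new notice widget to the viewport on each entry.
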(event `/Game/ThirdPerson/Blueprints/Interaction_Interface.Interaction`
  (params (Actor :type "Actor Object Reference"))
  (`GameplayStatics.PlaySound2D` "/Game/SoundEffect/SFX/Press.Press" 1.0 1.0 0.0 null null)
  (set `self.isCorrect?` true)
  (for (_array_element _array_index) (`self.Puzzle Pieces`)
    (if (!= (`/Game/Lighting_Game/BP_LightButton1.ColorIndex` _array_element) (`|GetArrayItem` (`self.Color Code`) _array_index))
      (set `self.isCorrect?` false)
      (break)))
  (if (`self.isCorrect?`)
    (`/Engine/EditorBlueprintResources/StandardMacros.DoOnce` false
      (:`Completed`
        (bind _doortoopen (`self.DoortoOpen`)
          (:`then`
            (if (`KismetSystemLibrary.DoesImplementInterface` _doortoopen "/Game/ThirdPerson/Blueprints/Interaction_Interface.Interaction_Interface_C")
              (message `/Game/ThirdPerson/Blueprints/Interaction_Interface.Interaction` _doortoopen self)
              (`GameplayStatics.PlaySound2D` "/Game/SoundEffect/SFX/Correct.Correct" 1.0 1.0 0.0 null null)))
          (:`else`))))
    (else
      (for _array_element_2 (`self.Puzzle Pieces`)
        (set `/Game/Lighting_Game/BP_LightButton1.ColorIndex` 0 _array_element_2)
        (`/Game/Lighting_Game/BP_LightButton1.Update Light Color` _array_element_2)
        (`GameplayStatics.PlaySound2D` "/Game/SoundEffect/SFX/Error.Error" 1.0 1.0 0.0 null null)))))

(event `self.Sphere.OnComponentBeginOverlap`
  (params (OverlappedComponent :type "PrimitiveComponent Object Reference") (OtherActor :type "Actor Object Reference") (OtherComp :type "PrimitiveComponent Object Reference") (OtherBodyIndex :type Integer) (bFromSweep :type Boolean) (SweepResult :type "HitResult Structure (by ref)"))
  (`SceneComponent.SetVisibility` (`self.Widget`) true false)
  (bind _returnvalue (`|CreateWidget` "/Game/UI/Notice_WB/WB_Notice_Button.WB_Notice_Button_C"))
  (`UserWidget.AddToViewport` _returnvalue 0))

(event `self.Sphere.OnComponentEndOverlap`
  (params (OverlappedComponent :type "PrimitiveComponent Object Reference") (OtherActor :type "Actor Object Reference") (OtherComp :type "PrimitiveComponent Object Reference") (OtherBodyIndex :type Integer))
  (`SceneComponent.SetVisibility` (`self.Widget`) false false))

(fn `UserConstructionScript`)