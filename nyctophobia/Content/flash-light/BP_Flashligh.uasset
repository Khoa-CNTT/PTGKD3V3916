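; BP_Flashligh is a flashlight pickup actor that the player collects through an Interaction event.
; On BeginPlay it caches the player's BP_FirstPersonCharacter, and a Sphere overlap shows or hides its Widget, with no filter on the overlapping actor.
; Interaction plays a pickup sound, calls GiveFlashlight on the cached character and destroys the actor.
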(event `self.ReceiveBeginPlay`
  (bind _asbp_first_person_character (cast `/Game/ThirdPerson/Blueprints/BP_FirstPersonCharacter` (`GameplayStatics.GetPlayerCharacter` 0)))
  (set `self.Character` _asbp_first_person_character))

(event `/Game/ThirdPerson/Blueprints/Interaction_Interface.Interaction`
  (`GameplayStatics.PlaySound2D` "/Game/SoundEffect/Picking_Flashlight.Picking_Flashlight" 1.0 1.0 0.0 null null)
  (`/Game/ThirdPerson/Blueprints/BP_FirstPersonCharacter.GiveFlashlight` (`self.Character`))
  (`self.K2_DestroyActor`))

(event `self.Sphere.OnComponentBeginOverlap`
  (params (OverlappedComponent :type "PrimitiveComponent Object Reference") (OtherActor :type "Actor Object Reference") (OtherComp :type "PrimitiveComponent Object Reference") (OtherBodyIndex :type Integer) (bFromSweep :type Boolean) (SweepResult :type "HitResult Structure (by ref)"))
  (bind _output_get (set `self.Widget` (`self.Widget`)))
  (`SceneComponent.SetVisibility` _output_get true false))

(event `self.Sphere.OnComponentEndOverlap`
  (params (OverlappedComponent :type "PrimitiveComponent Object Reference") (OtherActor :type "Actor Object Reference") (OtherComp :type "PrimitiveComponent Object Reference") (OtherBodyIndex :type Integer))
  (bind _output_get (set `self.Widget` (`self.Widget`)))
  (`SceneComponent.SetVisibility` _output_get false false))

(fn `UserConstructionScript`)