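; BP_Picture is an interactable picture puzzle piece whose frame the player rotates to a target position.
; Each interaction, unless finalized, runs a timeline that lerps the frame's pitch by -90 degrees with a sound, ignoring rotation requests while moving.
; When the turn ends, a position counter increments without wrapping; matching PuzzleAnswer finalizes the piece, plays a transition sound, spawns an explosion emitter and shows the Plane.
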(event `self.ReceiveBeginPlay`
  (set `self.Starting Rotate Frame` (`SceneComponent.RelativeRotation` (`self.PictureFrame`))))

(event `/Game/ThirdPerson/Blueprints/Interaction_Interface.Interaction`
  (params (Actor :type "Actor Object Reference"))
  (if (not (`self.Finalized`))
    (`self.Rotate Painting`)))

(event `Rotate Painting`
  (bind (_starting_rotate_frame_roll _starting_rotate_frame_pitch) (`KismetMathLibrary.BreakRotator` (`self.Starting Rotate Frame`)))
  (if (not (`self.FrameMoving`))
    (set `self.FrameMoving` true)
    (`GameplayStatics.PlaySound2D` "/Game/SoundEffect/Rotate_Sound.Rotate_Sound" 1.5 1.0 0.0 null null)
    (bind (_direction _rotation) (`Timeline|Painting Rotate` :!via `PlayFromStart`)
      (:`Update`
        (bind _returnvalue (`KismetMathLibrary.Lerp` _starting_rotate_frame_pitch (- _starting_rotate_frame_pitch 90.0) _rotation))
        (`SceneComponent.K2_SetRelativeRotation` (`self.PictureFrame`) (`KismetMathLibrary.MakeRotator` 0.0 _returnvalue) false false))
      (:`Finished`
        (set `self.Starting Rotate Frame` (`KismetMathLibrary.MakeRotator` 0.0 _returnvalue))
        (set `self.FrameMoving` false)
        (bind _result (`/Engine/EditorBlueprintResources/StandardMacros.IncrementInt` (`self.FramePosition`))
          (:`  `
            (set `self.FramePosition` _result)
            (if (== (`self.PuzzleAnswer`) (`self.FramePosition`))
              (`GameplayStatics.PlaySound2D` "/Game/SoundEffect/Transtion.Transtion" 1.0 1.0 0.0 null null)
              (set `self.Finalized` true)
              (`GameplayStatics.SpawnEmitterAttached` "/Game/StarterContent/Particles/P_Explosion.P_Explosion" (`self.Plane`) "None" (0.0 0.0 0.0) (struct) (1.0 1.0 1.0) "KeepRelativeOffset" false)
              (`SceneComponent.SetVisibility` (`self.Plane`) true false))))))))

(fn `UserConstructionScript`
  (`parent.UserConstructionScript`))