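; BP_ItemEnding is a collectible item that shows a widget while something overlaps its sphere.
; On Interaction it calls AddItem on the WB_MyGame game instance and plays a collect sound.
; It then swaps the mesh to a dissolve material, and a timeline animates the Dissolve parameter on a dynamic instance.
; When the timeline finishes, the actor destroys itself and adds a WB_Notice_Item widget to the viewport.
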(event `/Game/ThirdPerson/Blueprints/Interaction_Interface.Interaction`
  (params (Actor :type "Actor Object Reference"))
  (bind _staticmesh (`self.StaticMesh`))
  (bind _aswb_my_game (cast `/Game/SaveGame/WB_MyGame` (`GameplayStatics.GetGameInstance`)))
  (`/Game/SaveGame/WB_MyGame.AddItem` _aswb_my_game)
  (`GameplayStatics.PlaySound2D` "/Game/SoundEffect/SFX/Collect.Collect" 1.0 1.0 0.0 null null)
  (`PrimitiveComponent.SetMaterial` (`self.StaticMesh`) 0 "/Game/ThirdPerson/Blueprints/Dissolve_Mat_Inst.Dissolve_Mat_Inst")
  (bind _returnvalue (`PrimitiveComponent.CreateDynamicMaterialInstance` _staticmesh 0 (`PrimitiveComponent.GetMaterial` _staticmesh 0) "None"))
  (bind _output_get (set `self.CubeMaterial` _returnvalue))
  (bind (_direction _dissolvetrack) (`Timeline|Timeline` :!via `PlayFromStart`)
    (:`Update`
      (`MaterialInstanceDynamic.SetScalarParameterValue` _output_get "Dissolve" (`KismetMathLibrary.Lerp` -1.0 1.0 _dissolvetrack)))
    (:`Finished`
      (`self.K2_DestroyActor`)
      (bind _returnvalue_2 (`|CreateWidget` "/Game/UI/Notice_WB/WB_Notice_Item.WB_Notice_Item_C"))
      (`UserWidget.AddToViewport` _returnvalue_2 0))))

(event `self.Sphere.OnComponentBeginOverlap`
  (params (OverlappedComponent :type "PrimitiveComponent Object Reference") (OtherActor :type "Actor Object Reference") (OtherComp :type "PrimitiveComponent Object Reference") (OtherBodyIndex :type Integer) (bFromSweep :type Boolean) (SweepResult :type "HitResult Structure (by ref)"))
  (bind _output_get (set `self.Widget` (`self.Widget`)))
  (`SceneComponent.SetVisibility` _output_get true false))

(event `self.Sphere.OnComponentEndOverlap`
  (params (OverlappedComponent :type "PrimitiveComponent Object Reference") (OtherActor :type "Actor Object Reference") (OtherComp :type "PrimitiveComponent Object Reference") (OtherBodyIndex :type Integer))
  (bind _output_get (set `self.Widget` (`self.Widget`)))
  (`SceneComponent.SetVisibility` _output_get false false))

(fn `UserConstructionScript`)