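; BP_Door is an interactable door that swings open and closed, with optional key locking.
; Interaction toggles a Timeline-driven rotation, using a dot product against the right vector to pick swing direction.
; When locked, it checks the first-person character's Keys against DoorKeyID, then either unlocks and opens or shakes and spawns notice widgets.
; A Box overlap toggles a widget's visibility, and a Sound function selects lock, open or close audio.
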(event `self.ReceiveBeginPlay`
  (bind _asbp_first_person_character (cast `/Game/ThirdPerson/Blueprints/BP_FirstPersonCharacter` (`GameplayStatics.GetPlayerCharacter` 0)))
  (set `self.As BP First Person Character` _asbp_first_person_character))

(event `Open Close Door`
  ;[1 1 1] Open Close Door
  (`self.Sound`)
  (if (`self.DoorClosed?`)
    (set `self.DoorClosed?` false)
    (set `self.DotProduct` (`KismetMathLibrary.Dot_VectorVector` (`KismetMathLibrary.Normal` (- (`self.K2_GetActorLocation` self) (`self.K2_GetActorLocation`))) (`self.GetActorRightVector` self)))
    (bind (_direction _door) (`Timeline|Timeline` :!label _label)
      (:`Update`
        (`SceneComponent.K2_SetRelativeRotation` (`self.Door`) (`KismetMathLibrary.MakeRotator` 0.0 0.0 (`KismetMathLibrary.Lerp` 0.0 (`KismetMathLibrary.SelectFloat` -120.0 120.0 (>= (`self.DotProduct`) 0.0)) _door)) false false)))
    (else
      (set `self.DoorClosed?` true)
      (goto _label :!via `Reverse`))))

(event `/Game/ThirdPerson/Blueprints/Interaction_Interface.Interaction`
  (params (Actor :type "Actor Object Reference"))
  ;[1 1 1] Interaction
  (if (`self.Locked?`)
    (`self.Check Key`)
    (else
      (`self.Open Close Door`))))

(event `UnlockDoor`
  ;[1 1 1] Unlock Door
  (set `self.Locked?` false)
  (`GameplayStatics.PlaySoundAtLocation` "/Game/SoundEffect/SFX/Door_Unlock.Door_Unlock" (`SceneComponent.K2_GetComponentLocation` (`self.Door`)) (struct) 1.0 1.0 0.0 null null null null)
  (`KismetSystemLibrary.Delay` 0.2)
  (`self.Open Close Door`))

(event `Check Key`
  ;[1 1 1] Key Check
  (`self.Sound`)
  (for _array_element (`/Game/ThirdPerson/Blueprints/BP_FirstPersonCharacter.Keys` (`self.As BP First Person Character`))
    _)
  (if (`KismetTextLibrary.EqualEqual_TextText` _array_element (`self.DoorKeyID`))
    (`self.UnlockDoor`)
    (else
      (`self.Shake Door`))))

(event `Shake Door`
  ;[1 1 1] Door Shake
  (bind (_direction _newtrack_0) (`Timeline|ShakeDoorTL` :!via `PlayFromStart`)
    (:`Update`
      (`SceneComponent.K2_SetRelativeRotation` (`self.Door`) (`KismetMathLibrary.MakeRotator` 0.0 0.0 _newtrack_0) false false)
      (bind _returnvalue (`|CreateWidget` "/Game/UI/Notice_WB/WB_Notice_Door.WB_Notice_Door_C"))
      (`UserWidget.AddToViewport` _returnvalue 0))))

(event `self.Box.OnComponentBeginOverlap`
  (params (OverlappedComponent :type "PrimitiveComponent Object Reference") (OtherActor :type "Actor Object Reference") (OtherComp :type "PrimitiveComponent Object Reference") (OtherBodyIndex :type Integer) (bFromSweep :type Boolean) (SweepResult :type "HitResult Structure (by ref)"))
  ;[1 1 1] Widget
  (bind _output_get (set `self.Widget` (`self.Widget`)))
  (`SceneComponent.SetVisibility` _output_get true false))

(event `self.Box.OnComponentEndOverlap`
  (params (OverlappedComponent :type "PrimitiveComponent Object Reference") (OtherActor :type "Actor Object Reference") (OtherComp :type "PrimitiveComponent Object Reference") (OtherBodyIndex :type Integer))
  ;[1 1 1] Widget
  (bind _output_get (set `self.Widget` (`self.Widget`)))
  (`SceneComponent.SetVisibility` _output_get false false))

(fn `Sound`
  (bind _returnvalue (`SceneComponent.K2_GetComponentLocation` (`self.Door`)))
  (if (`self.Locked?`)
    (`GameplayStatics.PlaySoundAtLocation` (`self.LockSound`) _returnvalue (struct) 2.0 1.0 0.0 null null null null)
    (elif (`self.DoorClosed?`)
      (`GameplayStatics.PlaySoundAtLocation` (`self.Open Sound`) _returnvalue (struct) 1.0 1.0 0.0 null null null null)
      (else
        (`GameplayStatics.PlaySoundAtLocation` (`self.Close Sound`) _returnvalue (struct) 1.0 1.0 0.0 null null null null)))))

(fn `UserConstructionScript`)