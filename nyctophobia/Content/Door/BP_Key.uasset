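; BP_Key is a collectible key pickup that adds its KeyID to the first-person player character's keys.
; The construction script applies the KeyMesh variable to the static mesh, so each instance can have its own look.
; BeginPlay caches the player character.
; Interaction plays a collect sound, shows the WB_Notice_Key widget, passes the ID to AddKeys on the character and destroys the actor.
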(event `self.ReceiveBeginPlay`
  (bind _asbp_first_person_character (cast `/Game/ThirdPerson/Blueprints/BP_FirstPersonCharacter` (`GameplayStatics.GetPlayerCharacter` 0)))
  (set `self.As BP First Person Character` _asbp_first_person_character))

(event `/Game/ThirdPerson/Blueprints/Interaction_Interface.Interaction`
  (params (Actor :type "Actor Object Reference"))
  (`GameplayStatics.PlaySound2D` "/Game/SoundEffect/SFX/Collect.Collect" 1.0 1.0 0.0 null null)
  (bind _returnvalue (`|CreateWidget` "/Game/UI/Notice_WB/WB_Notice_Key.WB_Notice_Key_C"))
  (`UserWidget.AddToViewport` _returnvalue 0)
  (`/Game/ThirdPerson/Blueprints/BP_FirstPersonCharacter.AddKeys` (`self.As BP First Person Character`) (`self.KeyID`))
  (`self.K2_DestroyActor`))

(fn `UserConstructionScript`
  (`StaticMeshComponent.SetStaticMesh` (`self.StaticMesh`) (`self.KeyMesh`)))