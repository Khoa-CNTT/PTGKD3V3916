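; BP_Locker is an interactable locker that plays an opening animation and sound, apparently intended as a hiding spot.
; The Interaction event uses a DoOnce that resets after a short delay, blocking repeat triggers during the animation.
; A Sphere overlap shows and hides the interaction prompt widget.
; Box overlap events for entering and leaving the locker are empty stubs, so no hiding logic exists here.
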(event `/Game/ThirdPerson/Blueprints/Interaction_Interface.Interaction`
  (params (Actor :type "Actor Object Reference"))
  ;[1 1 1] Opens the locker
  (`/Engine/EditorBlueprintResources/StandardMacros.DoOnce` false :!label _label
    (:`Completed`
      (`GameplayStatics.PlaySound2D` "/Game/SoundEffect/SFX/LockerOpen.LockerOpen" 1.0 1.0 0.0 null null)
      (`SkeletalMeshComponent.PlayAnimation` (`self.SkeletalMesh`) "/Game/LockerHide/locker_rough_texture_Anim.locker_rough_texture_Anim" false)
      (`KismetSystemLibrary.Delay` 1.65)
      (goto _label :!via `Reset`))))

(event `self.Box.OnComponentBeginOverlap`
  (params (OverlappedComponent :type "PrimitiveComponent Object Reference") (OtherActor :type "Actor Object Reference") (OtherComp :type "PrimitiveComponent Object Reference") (OtherBodyIndex :type Integer) (bFromSweep :type Boolean) (SweepResult :type "HitResult Structure (by ref)"))
  ;[1 1 1] Event when player comes in the locker
)

(event `self.Box.OnComponentEndOverlap`
  (params (OverlappedComponent :type "PrimitiveComponent Object Reference") (OtherActor :type "Actor Object Reference") (OtherComp :type "PrimitiveComponent Object Reference") (OtherBodyIndex :type Integer))
  ;[1 1 1] Event when player goes out of the locker
)

(event `self.Sphere.OnComponentBeginOverlap`
  (params (OverlappedComponent :type "PrimitiveComponent Object Reference") (OtherActor :type "Actor Object Reference") (OtherComp :type "PrimitiveComponent Object Reference") (OtherBodyIndex :type Integer) (bFromSweep :type Boolean) (SweepResult :type "HitResult Structure (by ref)"))
  ;[1 1 1] UI Interact
  (`SceneComponent.SetVisibility` (`self.Widget`) true false))

(event `self.Sphere.OnComponentEndOverlap`
  (params (OverlappedComponent :type "PrimitiveComponent Object Reference") (OtherActor :type "Actor Object Reference") (OtherComp :type "PrimitiveComponent Object Reference") (OtherBodyIndex :type Integer))
  ;[1 1 1] UI Interact
  (`SceneComponent.SetVisibility` (`self.Widget`) false false))

(fn `UserConstructionScript`)